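; Main character Blueprint that performs a sword slice when the Slice input is pressed.
; The press spawns MySword_BP at the character's location and rotation if SliceTimer allows it.
; SliceTimer works as a short cooldown flag, set on the press and cleared by a Delay rather than counted down on Tick.
; Unconnected leftovers hold a gated repeat-shoot routine with no spawn class and a rotation debug print.
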(event `InputAction|Shoot`
  (params (Key :type "Key Structure")))

(event `InputAction|Slice`
  (params (Key :type "Key Structure"))
  (:`Pressed`
    (if (<= (`self.SliceTimer`) 0.0)
      (`|ExecutionSequence`
        (:`then_0`
          (`|SpawnActorFromClass` "/Game/Custom_BluePrints/MySword_BP.MySword_BP_C" (`KismetMathLibrary.MakeTransform` (`self.K2_GetActorLocation`) (`self.K2_GetActorRotation`)) "Undefined" "OverrideRootScale" null null)
          (`KismetSystemLibrary.Delay` 0.2)
          (set `self.SliceTimer` 0.0))
        (:`then_1`
          (set `self.SliceTimer` 0.2))))))

(event `self.ReceiveTick`
  (params (DeltaSeconds :type "Float (single-precision)")))

(fn `UserConstructionScript`)