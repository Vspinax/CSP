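; Short-lived boss laser actor, judging by its name, that animates its scale and destroys itself after a brief delay.
; Tick drives two Gates: the first, opened on BeginPlay, raises Size until it passes a threshold, which closes it and opens the second to lower Size more slowly.
; Both branches feed Size as uniform scale into a shared AddActorLocalTransform with zero translation and rotation.
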(event `self.ReceiveBeginPlay`
  (bind _size (`self.size`))
  (`|ExecutionSequence`
    (:`then_0`
      (set `self.size` 0.0)
      (`KismetSystemLibrary.Delay` 0.7)
      (`self.K2_DestroyActor`))
    (:`then_1`
      (goto _label :!via `Open`))))

(event `self.ReceiveTick`
  (params (DeltaSeconds :type "Float (single-precision)"))
  (bind _size (`self.size`))
  (`|ExecutionSequence`
    (:`then_0`
      (`/Engine/EditorBlueprintResources/StandardMacros.Gate` true :!label _label
        (:`Exit`
          (set `self.size` (+ (`self.size`) 1.0))
          (`self.K2_AddActorLocalTransform` (`KismetMathLibrary.MakeTransform` (0.0 0.0 0.0) (struct) (`KismetMathLibrary.MakeVector` _size _size _size)) :!label _label_2))))
    (:`then_1`
      (if (not (<= (`self.size`) 15.0))
        (`|ExecutionSequence`
          (:`then_0`
            (goto _label :!via `Close`))
          (:`then_1`
            (goto _label_3 :!via `Open`)))))
    (:`then_2`
      (`/Engine/EditorBlueprintResources/StandardMacros.Gate` true :!label _label_3
        (:`Exit`
          (set `self.size` (- (`self.size`) 0.25))
          (goto _label_2))))))

(fn `UserConstructionScript`)