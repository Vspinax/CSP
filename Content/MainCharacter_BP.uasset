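; MainCharacter_BP is the main character Blueprint, handling the Shoot and Slice input actions by spawning actors at its own location and rotation.
; Holding Shoot opens a Gate that loops through a 0.2-second Delay to spawn repeatedly until release closes it, though the spawn shows no class.
; Pressing Slice spawns a single Sword actor.
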(event `InputAction|Shoot`
  (params (Key :type "Key Structure"))
  (:`Pressed`
    (`|ExecutionSequence`
      (:`then_0`
        (goto _label :!via `Open`))
      (:`then_1`
        (`/Engine/EditorBlueprintResources/StandardMacros.Gate` true :!label _label
          (:`Exit`
            (`|SpawnActorFromClass` "/Game/MyBullet.MyBullet_C" (`KismetMathLibrary.MakeTransform` (`self.K2_GetActorLocation`) (`self.K2_GetActorRotation`) (1.0 1.0 1.0)) "Undefined" "OverrideRootScale" null null)
            (`KismetSystemLibrary.Delay` 0.2)
            (goto _label))))))
  (:`Released`
    (goto _label :!via `Close`)))

(event `InputAction|Slice`
  (params (Key :type "Key Structure"))
  (:`Pressed`
    (`|SpawnActorFromClass` "/Game/Sword.Sword_C" (`KismetMathLibrary.MakeTransform` (`self.K2_GetActorLocation`) (`self.K2_GetActorRotation`)) "Undefined" "OverrideRootScale" null null)))

(fn `UserConstructionScript`)