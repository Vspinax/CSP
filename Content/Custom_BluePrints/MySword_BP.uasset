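; Short-lived sword actor that spins around the player character's position, apparently as a quick swing attack, though it contains no hit or damage logic.
; On BeginPlay it takes its starting yaw from the player's rotation.
; Each Tick advances the yaw by a fixed, frame-rate-dependent step and snaps a component to the player's location with a zero-time MoveComponentTo.
; A Delay in the same Tick chain destroys the actor a fraction of a second later.
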(event `self.ReceiveBeginPlay`
  (set `self.rotation` (.yaw (`self.K2_GetActorRotation` (`GameplayStatics.GetPlayerCharacter` 0)))))

(event `self.ReceiveTick`
  (params (DeltaSeconds :type "Float (single-precision)"))
  (bind _output_get (set `self.rotation` (+ (`self.rotation`) 4.0)))
  (`KismetSystemLibrary.MoveComponentTo` null (`self.K2_GetActorLocation` (`GameplayStatics.GetPlayerCharacter` 0)) (`KismetMathLibrary.MakeRotator` 0.0 0.0 _output_get) false false 0.0)
  (`KismetSystemLibrary.Delay` 0.2)
  (`self.K2_DestroyActor`))

(fn `UserConstructionScript`)