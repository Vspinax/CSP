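; MainCharacter_BP is the main character Blueprint, with its attack logic currently disconnected.
; The only live logic prints a debug string when the Slice input is pressed or released.
; Unreachable graph fragments hold a timer-gated, Gate-driven repeating shot spawn with no class set, and an unfinished slice cooldown with a separate Sword_BP spawn.
; The construction script is empty.
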(event `InputAction|Shoot`
  (params (Key :type "Key Structure")))

(event `InputAction|Slice`
  (params (Key :type "Key Structure"))
  (:`Pressed`
    (`KismetSystemLibrary.PrintString` "WHAT" :!label _label))
  (:`Released`
    (goto _label)))

(fn `UserConstructionScript`)